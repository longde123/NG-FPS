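; Team deathmatch game state that wires components together to run a match from lobby through results.
; On gaining authority it seeds the spawner and scoreboard from TeamInfos, then relays kill, player and spawn-request events to scoring, counting and spawning components.
; Player count feeds the lobby timer, whose finish starts the match timer.
; Match end destroys NPCs and their spawners, with Spatial session state updated through Running, Results and, after a delay, Finished.
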(event KillEvent(ScorePublisher)
  (params (KillerState :type Player%20State%20Object%20Reference) (VictimState :type Player%20State%20Object%20Reference))
  ;[1 1 1] Publish Scores
  (CallFunction|OnKillEvent KillerState VictimState))

(event PlayerEvent(PlayerPublisher)
  (params (PlayerState :type Player%20State%20Object%20Reference) (Progress :type EPlayerProgress%20Enum :default "Connected"))
  ;[1 1 1] Listen to player events
  (Class|PlayerCountingComponent|PlayerEvent (Variables|Default|GetPlayerCounting) PlayerState Progress)
  (switch Utilities|FlowControl|Switch|SwitchonEPlayerProgress Progress
    (:InGame
      (Class|TeamDeathmatchScoreComponent|RecordNewPlayer (Variables|Default|GetTeamDeathmatchScore) PlayerState))
    (:Disconnected
      (Class|TeamDeathmatchScoreComponent|RemovePlayer (Variables|Default|GetTeamDeathmatchScore) PlayerState)
      (bind _asplayer_controller (Utilities|Casting|CastToPlayerController (Components|GetOwner PlayerState)))
      (Class|TeamDeathmatchSpawnerComponent|PlayerDisconnected (Variables|Default|GetTeamDeathmatchSpawner) _asplayer_controller))))

(event PlayerCountEvent(PlayerCounting)
  (params (PlayerCount :type Integer))
  ;[1 1 1] Start Lobby Countdown
  (Class|LobbyTimerComponent|ServerInformOfPlayerCount (Variables|Default|GetLobbyTimer) PlayerCount))

(event OnTimerFinished(LobbyTimer)
  ;[1 1 1] Start Match After Lobby
  (Class|MatchStateComponent|SetMatchState (Variables|Default|GetMatchState) "InGame")
  (Class|TimerComponent|StartTimer (Variables|Default|GetMatchTimer))
  (Class|SpatialSessionStateComponent|SendStateUpdate (Variables|Default|GetSpatialSessionState) "Running"))

(event OnTimerFinished(MatchTimer)
  ;[1 1 1] Finish Match
  (CallFunction|KillNPCs)
  (Class|MatchStateComponent|SetMatchState (Variables|Default|GetMatchState) "PostGame")
  (Class|SpatialSessionStateComponent|SendStateUpdate (Variables|Default|GetSpatialSessionState) "Results")
  (Utilities|FlowControl|Delay 6e+01)
  (Class|SpatialSessionStateComponent|SendStateUpdate (Variables|Default|GetSpatialSessionState) "Finished"))

(event OnSpawnRequest(SpawnRequestPublisher)
  (params (Controller :type Player%20Controller%20Object%20Reference))
  ;[1 1 1] Pass spawn requests to deathmatch spawner
  (Class|TeamDeathmatchSpawnerComponent|RequestSpawn (Variables|Default|GetTeamDeathmatchSpawner) Controller))

(event Custom|OnKillEvent
  (params (Killer%20State :type Player%20State%20Object%20Reference) (Victim%20State :type Player%20State%20Object%20Reference))
  (bind _returnvalue (Actor|GetComponentbyClass "/Script/GDKShooter.TeamComponent"))
  (bind _returnvalue_2 (Class|TeamComponent|GetTeam _returnvalue))
  ;[1 1 1] Publish Scores
  (Class|TeamDeathmatchScoreComponent|RecordKill (Variables|Default|GetTeamDeathmatchScore) Killer%20State Victim%20State)
  (Class|TeamDeathmatchScoreComponent|SetTeamScore (Variables|Default|GetTeamDeathmatchScore) _returnvalue_2 (+ (Class|TeamDeathmatchScoreComponent|GetTeamScore (Variables|Default|GetTeamDeathmatchScore) _returnvalue_2) 1))
  (Development|PrintText "Hello TDM"))

(event EventAuthorityGained
  (Class|TeamDeathmatchSpawnerComponent|SetTeams (Variables|Default|GetTeamDeathmatchSpawner) (CallFunction|ToTeamIds (Variables|Default|GetTeamInfos)))
  (Class|TeamDeathmatchScoreComponent|SetTeamScores (Variables|Default|GetTeamDeathmatchScore) (CallFunction|ToTeamScores (Variables|Default|GetTeamInfos))))

(fn ConstructionScript)

(fn ToTeamIds
  (params (TeamInfos :type Array%20of%20GDK%20Team%20Info%20Structures))
  (for _array_element TeamInfos
    (Utilities|Array|Add (LocalVariables|GetOutTeamIds) (.id _array_element)))
  (return (LocalVariables|GetOutTeamIds)))

(fn ToTeamScores
  (params (TeamInfos :type Array%20of%20GDK%20Team%20Info%20Structures))
  (for _array_element TeamInfos
    (Utilities|Array|Add (LocalVariables|GetOutTeamScores) (Utilities|Struct|MakeTeamScore (.id _array_element) (.name _array_element))))
  (return (LocalVariables|GetOutTeamScores)))

(fn KillNPCs
  (bind _outactors (Actor|GetAllActorsOfClass "/Game/Blueprints/NPCs/NPCSpawner.NPCSpawner_C"))
  (for _array_element _outactors
    (Actor|DestroyActor _array_element))
  (bind _outactors_2 (Actor|GetAllActorsOfClass "/Game/Blueprints/NPCs/Character_NPC.Character_NPC_C"))
  (for _array_element_2 _outactors_2
    (Actor|DestroyActor _array_element_2))
  (return))