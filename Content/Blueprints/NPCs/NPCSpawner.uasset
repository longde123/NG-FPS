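; Server-side NPC spawner, attached to a control point, that spawns waves of AI characters on a looping timer.
; On BeginPlay, if enabled, it caches PlayerStarts attached to its parent as spawn points.
; Each wave prunes invalid NPCs, then spawns at random points up to the per-wave and live caps.
; Each NPC gets its own possessing AI controller and the controlling team, or a fallback team if uncontrolled.
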(event Custom|SpawnWave
  (bind _output (CallFunction|RandomSpawnPoint))
  (bind _control_point (Variables|Default|GetControl%20Point))
  (bind _returnvalue (Transformation|GetActorTransform _output))
  ;[1 1 1] Spawn Wave of NPCs up to MaxSpawnedNPCs
  (CallFunction|RemoveInvalidNPCs)
  (for _index (range 1 (Math|Integer|Min(Integer) (Variables|Default|GetNPCsPerWave) (- (Variables|Default|GetMaxSpawnedNPCs) (Utilities|Array|Length (Variables|Default|GetSpawnedNPCs)))))
    (bind _returnvalue_2 (Game|SpawnActorfromClass "/Game/Blueprints/NPCs/Character_NPC.Character_NPC_C" (Math|Transform|MakeTransform (.location _returnvalue) (.rotation _returnvalue) "1,1,1") "AdjustIfPossibleButAlwaysSpawn" self (select (Default|IsControlled _control_point) (Variables|/Game/Blueprints/BP_ControlPoint.BP_ControlPoint_C|GetControllingTeam _control_point) (Variables|Default|GetUncontrolledTeam)) 0))
    (bind _returnvalue_3 (Game|SpawnActorfromClass (Variables|/Script/Engine.Pawn|GetAIControllerClass _returnvalue_2) (Transformation|GetActorTransform _returnvalue_2) "AlwaysSpawn" self 0))
    (Pawn|Possess _returnvalue_3 _returnvalue_2)
    (Utilities|Array|Add (Variables|Default|GetSpawnedNPCs) _returnvalue_2)
    (Class|GDKShooterFunctionLibrary|SetGenericTeamId _returnvalue_2 (Variables|/Game/Blueprints/NPCs/Character_NPC.Character_NPC_C|GetTeam _returnvalue_2))))

(event EventBeginPlay
  ;[1 1 1] If Authority & Enabled, Cache Spawn Points and Start Wave Timer.
  (Networking|SwitchHasAuthority
    (:Authority
      (if (Variables|Default|GetSpawningEnabled)
        (Utilities|Time|SetTimerbyEvent (EventDispatchers|CreateEvent :!event Custom|SpawnWave) (Variables|Default|GetWaveIntervalSeconds) true)
        (bind _filteredarray (Utilities|Array|FilterArray (Actor|GetAttachedActors (Actor|GetAttachParentActor) true) "/Script/Engine.PlayerStart"))
        (Variables|Default|SetSpawnPoints _filteredarray)
        (bind _asbp_control_point (Utilities|Casting|CastToBP_ControlPoint (Actor|GetAttachParentActor)))
        (Variables|Default|SetControl%20Point _asbp_control_point)))))

(fn ConstructionScript)

(fn RemoveInvalidNPCs
  (for _array_element (Variables|Default|GetSpawnedNPCs)
    (Utilities|IsValid _array_element
      (:Is%20Valid
        (Utilities|Array|Add (LocalVariables|GetLocal) _array_element))))
  (Variables|Default|SetSpawnedNPCs (LocalVariables|GetLocal)))

(fn RandomSpawnPoint
  (return (Utilities|Array|Get(acopy) (Variables|Default|GetSpawnPoints) (Math|Random|RandomIntegerinRange 0 (- (Utilities|Array|Length (Variables|Default|GetSpawnPoints)) 1)))))