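; Frag grenade launcher weapon Blueprint that cycles between firing modes, each with its own projectile class.
; ToggleMode advances the mode index with wraparound, and SetModeIndex stores it and picks the matching ProjectileClass from the Projectiles array.
; The index is RepNotify, so its OnRep swaps the SMTextFrag static mesh to show the current mode's name.
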(event Custom|SetModeIndex
  (params (NewIndex :type Integer))
  (bind _output_get (Variables|Default|SetCurrentModeIndex NewIndex))
  (Variables|Default|SetProjectileClass (Utilities|Array|Get(acopy) (Variables|Default|GetProjectiles) _output_get)))

(event EventToggleMode
  (CallFunction|SetModeIndex (Math|Integer|%(Integer) (+ (Variables|Default|GetCurrentModeIndex) 1) (Utilities|Array|Length (Variables|Default|GetProjectiles)))))

(fn ConstructionScript)

(fn OnRepCurrentModeIndex
  (Components|StaticMesh|SetStaticMesh (Variables|Default|GetSM_Text_Frag) (Utilities|Array|Get(acopy) (Variables|Default|GetModeNameMeshes) (Variables|Default|GetCurrentModeIndex))))