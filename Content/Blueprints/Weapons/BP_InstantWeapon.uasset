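; BP_InstantWeapon is a weapon Blueprint that handles the visuals of instant shots and customization.
; On each rendered shot it spawns a BP_BulletTracer from the effect socket to the impact, or out to max range on a miss, plus a colour-tinted muzzle flash.
; Customization metadata supplies the colours and weapon material; updates create a dynamic material instance and animate its cloak override through a timeline.
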(event Custom|Assign%20Material%20Event
  (params (WeaponMaterial :type Material%20Interface%20Object%20Reference) (WeaponColour :type Linear%20Color%20Structure))
  (bind _returnvalue (Rendering|Material|CreateDynamicMaterialInstance (Variables|Character|GetMesh) 1 WeaponMaterial "None" :!class /Script/Engine.PrimitiveComponent))
  (Rendering|Material|SetVectorParameterValue _returnvalue "Cloak_Colour" WeaponColour :!class /Script/Engine.MaterialInstanceDynamic)
  (bind _cloakoverride (Timeline|Cloak_Timeline Play)
    (:Update
      (Rendering|Material|SetScalarParameterValue _returnvalue "Cloak_Override" _cloakoverride :!class /Script/Engine.MaterialInstanceDynamic))))

(event EventOnRenderShot
  (params (Location :type Vector :default "0, 0, 0") (bImpact :type Boolean))
  (bind _effectsocketname (Variables|Default|GetEffectSocketName))
  (bind _mesh (Variables|Character|GetMesh))
  (bind _metadataprovider (Variables|Default|GetMetaDataProvider))
  (bind _metadata (Variables|Default|GetMetaData))
  (bind _returnvalue (Transformation|GetSocketLocation _mesh _effectsocketname))
  (bind _meta_data (Default|GetMetaData _metadataprovider (.customization _metadata)))
  (Game|SpawnActorfromClass "/Game/VFX/BP_BulletTracer.BP_BulletTracer_C" (Transformation|GetActorTransform) "Undefined" 0 _returnvalue (select bImpact Location (+ (* (Math|Vector|Normalize (- Location _returnvalue)) (Variables|/Script/GDKShooter.ShootingComponent|GetMaxRange (Class|Weapon|GetShootingComponent))) _returnvalue)) (Variables|Default|GetBulletSpeed) bImpact (.customization (Variables|Default|GetMetaData)) (Transformation|GetVelocity (Components|GetOwner (Transformation|GetAttachParent (Variables|Transformation|GetRootComponent)))) (Variables|Default|GetTracerMaterial) 0)
  (bind _returnvalue_2 (Effects|SpawnEmitterAttached (Variables|Default|GetMuzzle%20VFX) (Variables|Character|GetMesh) (Variables|Default|GetEffectSocketName) "0, 0, 0" "90.000000, 0,0.000000"))
  (Utilities|IsValid _returnvalue_2
    (:Is%20Valid
      (Effects|Components|ParticleSystem|SetColorParameter _returnvalue_2 "MuzzleFront" (.particlecolour _meta_data))
      (Effects|Components|ParticleSystem|SetColorParameter _returnvalue_2 "MuzzleSide" (.particlecolour _meta_data))
      (Effects|Components|ParticleSystem|SetColorParameter _returnvalue_2 "MuzzleSparks" (.particlecolour _meta_data)))))

(event EventOnMetaDataUpdated
  (bind _metadataprovider (Variables|Default|GetMetaDataProvider))
  (bind _metadata (Variables|Default|GetMetaData))
  (bind _meta_data (Default|GetMetaData _metadataprovider (.customization _metadata)))
  (CallFunction|AssignMaterialEvent (.blockoutmaterial _meta_data) (.particlecolour _meta_data)))

(fn ConstructionScript)