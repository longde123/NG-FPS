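; Game state for the Takeover prototype mode, where teams score by holding control points instead of by kills.
; On gaining authority it gathers all control points, binds to team changes and tallies each team's points that are connected to a base.
; A looping timer adds score per controlled point, while kills are only recorded.
; Reaching the max score kills NPCs, enters post-game and sends Spatial session results, then Finished after a delay.
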(event Custom|OnMaxScoreReached
  ;[1 1 1] Max Score Reached
  (CallFunction|KillNPCs)
  (Class|MatchStateComponent|SetMatchState (Variables|Default|GetMatchState) "PostGame")
  (Class|SpatialSessionStateComponent|SendStateUpdate (Variables|Default|GetSpatialSessionState) "Results")
  (Utilities|FlowControl|Delay 6e+01)
  (Class|SpatialSessionStateComponent|SendStateUpdate (Variables|Default|GetSpatialSessionState) "Finished"))

(event EventOnKillEvent
  (params (Killer%20State :type Player%20State%20Object%20Reference) (Victim%20State :type Player%20State%20Object%20Reference))
  ;[1 1 1] Override default kill handling to avoid setting TeamScore
  (Class|TeamDeathmatchScoreComponent|RecordKill (Variables|Default|GetTeamDeathmatchScore) Killer%20State Victim%20State))

(event EventAuthorityGained
  (|CallParentFunction)
  (Utilities|FlowControl|Sequence
    (:then_0
      ;[1 1 1] Find all control points in the map and update team scores when they change control
      (bind _outactors (Actor|GetAllActorsOfClass "/Game/TakeoverPrototype/BP_Takeover_ControlPoint.BP_Takeover_ControlPoint_C"))
      (for _array_element _outactors
        (Utilities|Array|Add (Variables|Default|GetControlPoints) _array_element)
        (EventDispatchers|BindEventtoOnControllingTeamChanged _array_element (EventDispatchers|CreateEvent :!event UpdateControlledPoints)))
      (CallFunction|UpdateControlledPoints))
    (:then_1
      (Utilities|Time|SetTimerbyEvent (EventDispatchers|CreateEvent :!event UpdateScores) (Variables|Default|GetUpdateScoresInterval) true))))

(fn ConstructionScript
  (|CallParentFunction))

(fn UpdateControlledPoints
  (for _array_element (Variables|Default|GetTeamInfos)
    (Utilities|Array|Add (LocalVariables|GetLocalControlledPoints) 0))
  (for _array_element_2 (Variables|Default|GetControlPoints)
    ;[1 1 1] Gets amount of controlled points per team
    (if (>= (Utilities|Array|FindItem (CallFunction|ToTeamIds (Variables|Default|GetTeamInfos)) (Variables|/Game/TakeoverPrototype/BP_Takeover_ControlPoint.BP_Takeover_ControlPoint_C|GetControllingTeam _array_element_2)) 0)
      ;;[1 1 1] Check if Control Point is connected to main base
      (if (Variables|/Game/TakeoverPrototype/BP_Takeover_ControlPoint.BP_Takeover_ControlPoint_C|GetIsConnectedToBase _array_element_2)
        (Utilities|Array|SetArrayElem (LocalVariables|GetLocalControlledPoints) (Utilities|Array|FindItem (CallFunction|ToTeamIds (Variables|Default|GetTeamInfos)) (Variables|/Game/TakeoverPrototype/BP_Takeover_ControlPoint.BP_Takeover_ControlPoint_C|GetControllingTeam _array_element_2)) (+ (Utilities|Array|Get(acopy) (LocalVariables|GetLocalControlledPoints) (Utilities|Array|FindItem (CallFunction|ToTeamIds (Variables|Default|GetTeamInfos)) (Variables|/Game/TakeoverPrototype/BP_Takeover_ControlPoint.BP_Takeover_ControlPoint_C|GetControllingTeam _array_element_2))) 1) true))))
  (Variables|Default|SetControlledPoints (LocalVariables|GetLocalControlledPoints)))

(fn UpdateScores
  (for (_array_element _array_index) (Variables|Default|GetTeamInfos)
    (Development|PrintString (Utilities|String|ToString(Integer) (+ (Class|TeamDeathmatchScoreComponent|GetTeamScore (Variables|Default|GetTeamDeathmatchScore) (.id _array_element)) (* (Utilities|Array|Get(acopy) (Variables|Default|GetControlledPoints) _array_index) (Variables|Default|GetPointsPerControlPoint)))))
    (Class|TeamDeathmatchScoreComponent|SetTeamScore (Variables|Default|GetTeamDeathmatchScore) (.id _array_element) (+ (Class|TeamDeathmatchScoreComponent|GetTeamScore (Variables|Default|GetTeamDeathmatchScore) (.id _array_element)) (* (Utilities|Array|Get(acopy) (Variables|Default|GetControlledPoints) _array_index) (Variables|Default|GetPointsPerControlPoint))))
    (if (>= (+ (Class|TeamDeathmatchScoreComponent|GetTeamScore (Variables|Default|GetTeamDeathmatchScore) (.id _array_element)) (* (Utilities|Array|Get(acopy) (Variables|Default|GetControlledPoints) _array_index) (Variables|Default|GetPointsPerControlPoint))) (Variables|Default|GetMaxTeamScore))
      (LocalVariables|SetMaxScoreReached true)))
  (if (LocalVariables|GetMaxScoreReached)
    (CallFunction|OnMaxScoreReached)))