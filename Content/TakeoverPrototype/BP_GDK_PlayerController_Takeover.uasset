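; Player controller for a GDK team deathmatch takeover prototype, handling game joining, respawn, kill publishing and menus for login, pause, scoreboard and results.
; On each new pawn it binds aiming and shot events to scale turn speed and play timeline-driven recoil with camera shake.
; Debug-style keys possess a nearby IFV or tell the AI spawner to spawn waves or take over.
; A looping local timer line-traces for hoverable actors.
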(event DeathEvent(ControllerEvents)
  (params (Controller :type Controller%20Object%20Reference))
  (bind _returnvalue (Game|GetGameState))
  (bind _playerstate (Variables|/Script/Engine.Controller|GetPlayerState Controller))
  (bind _returnvalue_2 (Actor|GetComponentbyClass _returnvalue "/Script/GDKShooter.ScorePublisher"))
  ;[1 1 1] On Death, UnPosses and Publish the Kill
  (Pawn|UnPossess)
  (Utilities|IsValid _returnvalue_2
    (:Is%20Valid
      (Utilities|IsValid Controller
        (:Is%20Valid
          (Utilities|IsValid _playerstate
            (:Is%20Valid
              (Class|ScorePublisher|PublishKill _returnvalue_2 _playerstate (Variables|Default|GetPlayerState)))))))))

(event Custom|OnMatchEvent
  (params (CurrentState :type EMatchState%20Enum :default "PreGame"))
  ;[1 1 1] Listen for match ending and display results UI
  (if (Utilities|Enum|Equal(Enum) CurrentState "PostGame")
    (Class|GDKPlayerController|SetUIMode true)
    (Default|RequestMenu (Variables|Default|GetMenuMediator) "NewEnumerator5")))

(event Custom|OnAiming
  (params (bIsAiming :type Boolean))
  (bind _output_get (Variables|Default|SetIsAiming bIsAiming))
  (CallFunction|AdjustTurnSpeedsforAiming _output_get))

(event Custom|OnShot
  (params (Weapon :type Weapon%20Object%20Reference) (Hit :type Boolean))
  (bind _isaiming (Variables|Default|GetIsAiming))
  (bind _recoilshake (Variables|/Script/GDKShooter.Weapon|GetRecoilShake Weapon))
  (bind _recoilaimmodifier (Variables|/Script/GDKShooter.Weapon|GetRecoilAimModifier Weapon))
  (bind _returnvalue (Math|Float|SelectFloat _recoilaimmodifier 1.0 _isaiming))
  ;[1 1 1] On Shot: Play Recoil and Camera Shake
  (Utilities|IsValid Weapon
    (:Is%20Valid
      (Components|Timeline|SetPlayRate (Variables|Default|GetRecoil) (Variables|/Script/GDKShooter.Weapon|GetRecoilRecoveryRate Weapon))
      (CallFunction|CalculateRecoilValues Weapon)
      (if (Utilities|IsValidClass _recoilshake)
        (Class|PlayerController|ClientPlayCameraShake _recoilshake 1.0 "CameraLocal" "0, 0, 0")
        (bind _lerp (Timeline|Recoil PlayFromStart)
          (:Update
            (Class|PlayerController|AddYawInput (* (Math|Float|Lerp (Variables|Default|GetRecoilYaw) 0.0 _lerp) _returnvalue))
            (Class|PlayerController|AddPitchInput (* (Math|Float|Lerp (Variables|Default|GetRecoilPitch) 0.0 _lerp) _returnvalue))))
        (else
          (Timeline|Recoil PlayFromStart))))))

(event Custom|Spawn%20AI
  (params (NewParam :type Player%20State%20Object%20Reference))
  (bind _outactors (Actor|GetAllActorsOfClass "/Game/TakeoverPrototype/AI_Spawner.AI_Spawner_C"))
  (Default|SpawnWave (Utilities|Array|Get(acopy) _outactors) NewParam))

(event Custom|Takeover
  (params (NewParam :type Player%20State%20Object%20Reference))
  (bind _outactors (Actor|GetAllActorsOfClass "/Game/TakeoverPrototype/AI_Spawner.AI_Spawner_C"))
  (Default|Takeover (Utilities|Array|Get(acopy) _outactors) NewParam))

(event Custom|HoverCheck
  (bind _shootingcomponent (Variables|Default|GetShootingComponent))
  (bind _returnvalue (Class|ShootingComponent|GetLineTraceDirection _shootingcomponent))
  (bind _returnvalue_2 (Class|ShootingComponent|DoLineTrace _shootingcomponent _returnvalue 0))
  ;[1 1 1] Raycast for IHover implementations
  (Utilities|IsValid _shootingcomponent
    (:Is%20Valid
      (Utilities|IsValid (.hitactor _returnvalue_2)
        (:Is%20Valid
          (bind _asbpi_on_hover (Utilities|Casting|CastToBPI_OnHover (.hitactor _returnvalue_2)))
          (Default|OnHover _asbpi_on_hover))))))

(event Custom|VehicleTakeover
  (params (Controller :type BP%20GDK%20Player%20Controller%20Takeover%20Object%20Reference))
  (bind _returnvalue (Pawn|GetControlledPawn Controller))
  (bind _outactors (Actor|GetAllActorsOfClass "/Game/OWIContent/Vehicles/LAVIFV/BP_LAVIFV.BP_LAVIFV_C"))
  (bind _output_get (Variables|Default|SetClosestIFV (Utilities|Array|Get(acopy) _outactors)))
  (for _array_element _outactors
    (if (> (Variables|Default|GetEnteringDistance) (Math|Vector|VectorLength (- (Transformation|GetActorLocation _array_element) (Transformation|GetActorLocation _returnvalue))))
      (if (> (Math|Vector|VectorLength (- (Transformation|GetActorLocation _output_get) (Transformation|GetActorLocation _returnvalue))) (Math|Vector|VectorLength (- (Transformation|GetActorLocation _array_element) (Transformation|GetActorLocation _returnvalue))))
        (Variables|Default|SetClosestIFV _array_element))))
  (Pawn|UnPossess Controller)
  (Pawn|Possess Controller _output_get))

(event EventTick
  (params (DeltaSeconds :type Float%20%28single-precision%29))
  (bind _returnvalue (Game|GetGameState))
  (bind _returnvalue_2 (Actor|GetComponentbyClass _returnvalue "/Script/GDKShooter.DeathmatchSpawnerComponent"))
  (bind _returnvalue_3 (Actor|GetComponentbyClass _returnvalue "/Script/GDKShooter.MatchStateComponent"))
  ;[1 1 1] Begin Play
  (if (Variables|Default|GetTryJoinGame)
    (Utilities|IsValid _returnvalue_2
      (:Is%20Valid
        (bind _returnvalue_4 (Class|DeathmatchSpawnerComponent|IsSpawningEnabled _returnvalue_2))
        (if _returnvalue_4
          (Variables|Default|SetTryJoinGame false :!label _label)
          (Class|GDKPlayerController|ServerTryJoinGame)
          (else
            (Variables|Default|SetTryJoinGame true :!label _label_2))))
      (:Is%20Not%20Valid
        (Utilities|IsValid _returnvalue_3
          (:Is%20Valid
            (if (Utilities|Enum|Equal(Enum) (Class|MatchStateComponent|GetCurrentState _returnvalue_3) "InGame")
              (goto _label)
              (else
                (goto _label_2)))))))))

(event EventBeginPlay
  (bind _returnvalue (Game|GetGameState))
  (bind _returnvalue_2 (Game|GetGameState))
  (bind _playercameramanager (Variables|Default|GetPlayerCameraManager))
  (bind _menumediator (Variables|Default|GetMenuMediator))
  (bind _returnvalue_3 (Actor|GetComponentbyClass _returnvalue "/Script/GDKShooter.DeathmatchSpawnerComponent"))
  (bind _returnvalue_4 (Actor|GetComponentbyClass _returnvalue "/Script/GDKShooter.MatchStateComponent"))
  (bind _returnvalue_5 (Actor|GetComponentbyClass _returnvalue_2 "/Script/GDKShooter.SpawnRequestPublisher"))
  ;[1 1 1] Begin Play
  (Input|EnableInput 0)
  (if (Pawn|IsLocalPlayerController)
    (Utilities|Time|SetTimerbyEvent (delegate Custom|HoverCheck) 0.2 true))
  (Variables|/Script/Engine.PlayerCameraManager|SetDefaultFOV (Variables|Default|GetPlayerCameraManager) 55.0)
  (Variables|/Script/Engine.PlayerCameraManager|SetViewPitchMax _playercameramanager (Variables|Default|GetMax%20Pitch))
  (Variables|/Script/Engine.PlayerCameraManager|SetViewPitchMin _playercameramanager (Variables|Default|GetMin%20Pitch))
  (Utilities|IsValid _returnvalue_5
    (:Is%20Valid
      (if (and (or (Variables|/Script/GDKShooter.SpawnRequestPublisher|GetbAutoConnect _returnvalue_5) (Class|SimPlayerBPFunctionLibrary|IsSimulatedPlayer)) (not (Networking|IsDedicatedServer)))
        (Default|RequestMenu _menumediator "NewEnumerator7")
        (Class|GDKPlayerController|SetUIMode false)
        (Utilities|FlowControl|Delay 0.2)
        (Utilities|IsValid _returnvalue_3
          (:Is%20Valid
            (bind _returnvalue_6 (Class|DeathmatchSpawnerComponent|IsSpawningEnabled _returnvalue_3))
            (if _returnvalue_6
              (Variables|Default|SetTryJoinGame false :!label _label)
              (Class|GDKPlayerController|ServerTryJoinGame)
              (else
                (Variables|Default|SetTryJoinGame true :!label _label_2))))
          (:Is%20Not%20Valid
            (Utilities|IsValid _returnvalue_4
              (:Is%20Valid
                (if (Utilities|Enum|Equal(Enum) (Class|MatchStateComponent|GetCurrentState _returnvalue_4) "InGame")
                  (goto _label)
                  (else
                    (goto _label_2)))))))
        (else
          (Default|RequestMenu _menumediator "NewEnumerator3")
          (Class|GDKPlayerController|SetUIMode true))))
    (:Is%20Not%20Valid
      (Development|PrintString "GDKPlayerController requires a SpawnRequestComponent on the GameState" false true "(R=1.000000,G=0.024069,B=0.000000,A=1.000000)" 2e+01))))

(event EventOnNewPawn
  (params (InPawn :type Pawn%20Object%20Reference))
  (bind _menumediator (Variables|Default|GetMenuMediator))
  ;[1 1 1] Bind Events on New Pawn
  (Utilities|IsValid InPawn
    (:Is%20Valid
      (Utilities|FlowControl|Sequence
        (:then_0
          (bind _output_get (Variables|Default|SetMovement (Actor|GetComponentbyClass InPawn "/Script/GDKShooter.GDKMovementComponent")))
          (Utilities|IsValid _output_get
            (:Is%20Valid
              (EventDispatchers|BindEventtoOnAimingUpdated (Variables|Default|GetMovement) (delegate Custom|OnAiming)))))
        (:then_1
          (bind _output_get_2 (Variables|Default|SetShootingComponent (Actor|GetComponentbyClass InPawn "/Script/GDKShooter.ShootingComponent")))
          (Utilities|IsValid _output_get_2
            (:Is%20Valid
              (EventDispatchers|BindEventtoShotEvent (Variables|Default|GetShootingComponent) (delegate Custom|OnShot)))))
        (:then_2
          (Default|RequestMenu (Variables|Default|GetMenuMediator) "NewEnumerator7")
          (Class|GDKPlayerController|SetUIMode false))
        (:then_3
          ;[1 1 1] Listen for match ending and display results UI
          (bind _asbp_team_deathmatch_game_state (Utilities|Casting|CastToBP_TeamDeathmatchGameState (Game|GetGameState)))
          (EventDispatchers|BindEventtoMatchEvent (Variables|/Game/GameMode/BP_TeamDeathmatchGameState.BP_TeamDeathmatchGameState_C|GetMatchState _asbp_team_deathmatch_game_state) (delegate Custom|OnMatchEvent)))))
    (:Is%20Not%20Valid
      (if (Utilities|Enum|NotEqual(Enum) (Default|GetLatestMenuRequest _menumediator) "NewEnumerator3")
        (Default|RequestMenu _menumediator "NewEnumerator4")
        (Class|GDKPlayerController|SetUIMode true)))))

(event Input|KeyboardEvents|SpaceBar
  (params (Key :type Key%20Structure :default "None"))
  ;[1 1 1] Space to respawn.  Unsure why we have to manually pass through jump here
  (:Pressed
    (if (Utilities|IsValid (Pawn|GetControlledPawn))
      (bind _ascharacter (Utilities|Casting|CastToCharacter (Pawn|GetControlledPawn)))
      (Character|Jump _ascharacter)
      (else
        (Class|GDKPlayerController|ServerRespawnCharacter)
        (Variables|Default|SetInputYawScale (Variables|Default|GetBaseYawScale))
        (Variables|Default|SetInputPitchScale (Variables|Default|GetBasePitchScale))))))

(event Input|KeyboardEvents|B
  (params (Key :type Key%20Structure :default "None"))
  (:Pressed
    (CallFunction|SpawnAI (Variables|Default|GetPlayerState))))

(event Input|KeyboardEvents|Escape
  (params (Key :type Key%20Structure :default "None"))
  (bind _menumediator (Variables|Default|GetMenuMediator))
  ;[1 1 1] In-game menu
  (:Pressed
    (switch Utilities|FlowControl|Switch|SwitchonMenus (Default|GetLatestMenuRequest _menumediator)
      (:NewEnumerator7
        (Default|RequestMenu _menumediator "NewEnumerator1")
        (Class|GDKPlayerController|SetUIMode true))
      (:NewEnumerator1
        (Default|RequestMenu _menumediator "NewEnumerator7")
        (Class|GDKPlayerController|SetUIMode false)))))

(event Input|KeyboardEvents|Tab
  (params (Key :type Key%20Structure :default "None"))
  (bind _menumediator (Variables|Default|GetMenuMediator))
  (bind _menumediator_2 (Variables|Default|GetMenuMediator))
  ;[1 1 1] In-game scoreboard
  (:Pressed
    (if (Utilities|Enum|Equal(Enum) (Default|GetLatestMenuRequest _menumediator_2) "NewEnumerator7")
      (Default|RequestMenu _menumediator_2 "NewEnumerator0")))
  (:Released
    (if (Utilities|Enum|Equal(Enum) (Default|GetLatestMenuRequest _menumediator) "NewEnumerator0")
      (Default|RequestMenu _menumediator "NewEnumerator7"))))

(event Input|KeyboardEvents|V
  (params (Key :type Key%20Structure :default "None"))
  (:Pressed
    (CallFunction|Takeover (Variables|Default|GetPlayerState))))

(event Input|KeyboardEvents|F10
  (params (Key :type Key%20Structure :default "None"))
  (bind _menumediator (Variables|Default|GetMenuMediator))
  ;[1 1 1] In-game menu
  (:Pressed
    (switch Utilities|FlowControl|Switch|SwitchonMenus (Default|GetLatestMenuRequest _menumediator)
      (:NewEnumerator7
        (Default|RequestMenu _menumediator "NewEnumerator1")
        (Class|GDKPlayerController|SetUIMode true))
      (:NewEnumerator1
        (Default|RequestMenu _menumediator "NewEnumerator7")
        (Class|GDKPlayerController|SetUIMode false)))))

(event Input|KeyboardEvents|C
  (params (Key :type Key%20Structure :default "None"))
  (:Pressed
    (CallFunction|VehicleTakeover self)))

(fn ConstructionScript
  (Variables|Default|SetBaseYawScale (Variables|Default|GetInputYawScale))
  (Variables|Default|SetBasePitchScale (Variables|Default|GetInputPitchScale)))

(fn CalculateRecoilValues
  (params (Weapon :type Weapon%20Object%20Reference))
  (bind _recoilcrouchmodifier (Variables|/Script/GDKShooter.Weapon|GetRecoilCrouchModifier Weapon))
  (bind _result (Math|Float|NegateFloat (Utilities|RecoilValue (Variables|/Script/GDKShooter.Weapon|GetRecoilPitchMax Weapon) (Variables|/Script/GDKShooter.Weapon|GetRecoilPitchMin Weapon) (Variables|/Script/GDKShooter.Weapon|GetRecoilUpBias Weapon)))
    (:%20%20
      (Variables|Default|SetRecoilPitch _result)
      (Variables|Default|SetRecoilYaw (Utilities|RecoilValue (Variables|/Script/GDKShooter.Weapon|GetRecoilYawMax Weapon) (Variables|/Script/GDKShooter.Weapon|GetRecoilYawMin Weapon) (Variables|/Script/GDKShooter.Weapon|GetRecoilRightBias Weapon)))
      ;[1 1 1] Dampen Recoil When Crouching
      (Utilities|IsCrouching
        (:ExecCrouching
          (Variables|Default|SetRecoilYaw (* (Variables|Default|GetRecoilYaw) _recoilcrouchmodifier))
          (Variables|Default|SetRecoilPitch (* (Variables|Default|GetRecoilPitch) _recoilcrouchmodifier)))))))

(fn AdjustTurnSpeedsforAiming
  (params (IsAiming :type Boolean))
  (bind _movement (Variables|Default|GetMovement))
  (bind _baseyawscale (Variables|Default|GetBaseYawScale))
  (bind _basepitchscale (Variables|Default|GetBasePitchScale))
  (bind _returnvalue (Class|GDKMovementComponent|GetAimingRotationModifier _movement))
  (Variables|Default|SetInputYawScale (Math|Float|SelectFloat (* _returnvalue _baseyawscale) _baseyawscale IsAiming))
  (Variables|Default|SetInputPitchScale (Math|Float|SelectFloat (* _returnvalue _basepitchscale) _basepitchscale IsAiming)))