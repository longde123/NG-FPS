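; BP_FPS_Character_Takeover is a prototype FPS character Blueprint with debug keys for testing tagging and fortification building.
; Z passes the character to TagTest, which calls AddTestTag on it and prints that a test tag component was added on the server.
; J spawns a Fortification1 at a fixed location and calls Place on it, while K places a buildable through BuildManager's ServerPlaceBuildable.
; BeginPlay and construction defer to the parent class.
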(event Custom|testSpawn
  (bind _returnvalue (Game|SpawnActorfromClass "/Game/TakeoverPrototype/Building/Fortification1.Fortification1_C" (Math|Transform|MakeTransform (Math|Vector|MakeVector 0.0 0.0 1.5e+02) "0, 0, 0" "1,1,1") "AdjustIfPossibleButAlwaysSpawn" 0 0))
  (Class|Buildable|Place _returnvalue))

(event Custom|TagTest
  (params (NewParam :type BP%20FPS%20Character%20Takeover%20Object%20Reference))
  ;[1 1 1] WORKS
  (AddComponent|AddTestTag NewParam)
  (Development|PrintString "Added Test Tag Component on Server during runtime"))

(event EventBeginPlay
  ;[1 1 1] WORKS
  (|CallParentFunction))

(event Collision|EventActorBeginOverlap
  (params (OtherActor :type Actor%20Object%20Reference)))

(event EventTick
  (params (DeltaSeconds :type Float%20%28single-precision%29)))

(event Input|KeyboardEvents|J
  (params (Key :type Key%20Structure :default "None"))
  (:Pressed
    (CallFunction|TestSpawn)))

(event Input|KeyboardEvents|K
  (params (Key :type Key%20Structure :default "None"))
  (:Pressed
    (Class|BuildManagerComponent|ServerPlaceBuildable (Variables|Default|GetBuildManager) (Math|Vector|MakeVector 0.0 0.0 1e+02) (Math|Rotator|MakeRotator 0.0 0.0 0.0))))

(event Input|KeyboardEvents|Z
  (params (Key :type Key%20Structure :default "None"))
  ;[1 1 1] WORKS
  (:Pressed
    (CallFunction|TagTest self)))

(fn ConstructionScript
  (|CallParentFunction))