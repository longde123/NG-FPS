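; Capturable control point for a team Takeover mode, which passes its controlling team to attached actors such as player starts.
; An authority-only looping timer drives a state machine from teams overlapping the Box: taking, removing or holding control, with delayed, proportional progress reset.
; Mixed teams mark it contested and pause progress.
; OnRep tints dynamic materials by team; local players inside see a progress widget until exit or death.
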(event OnComponentBeginOverlap(Box)
  (params (OverlappedComponent :type Primitive%20Component%20Object%20Reference) (OtherActor :type Actor%20Object%20Reference) (OtherComp :type Primitive%20Component%20Object%20Reference) (OtherBodyIndex :type Integer) (bFromSweep :type Boolean) (SweepResult :type Hit%20Result%20Structure%20%28by%20ref%29))
  (bind _aspawn (Utilities|Casting|CastToPawn OtherActor))
  (bind _asplayer_controller (Utilities|Casting|CastToPlayerController (Pawn|GetController _aspawn)))
  (if (Pawn|IsLocalPlayerController _asplayer_controller)
    (bind _returnvalue (UserInterface|CreateWidget "/Game/UI/Blueprints/BP_ControlPointProgress.BP_ControlPointProgress_C" _asplayer_controller self))
    (bind _output_get (Variables|Default|SetLocalPlayerUI _returnvalue))
    (UserInterface|Viewport|AddtoPlayerScreen _output_get)
    (Utilities|IsValid (Actor|GetComponentbyClass _aspawn "/Script/GDKShooter.HealthComponent")
      (:Is%20Valid
        (EventDispatchers|BindEventtoDeath (Actor|GetComponentbyClass _aspawn "/Script/GDKShooter.HealthComponent") (delegate Custom|OnDeath))))))

(event OnComponentEndOverlap(Box)
  (params (OverlappedComponent :type Primitive%20Component%20Object%20Reference) (OtherActor :type Actor%20Object%20Reference) (OtherComp :type Primitive%20Component%20Object%20Reference) (OtherBodyIndex :type Integer))
  (bind _localplayerui (Variables|Default|GetLocalPlayerUI))
  (bind _aspawn (Utilities|Casting|CastToPawn OtherActor))
  (bind _asplayer_controller (Utilities|Casting|CastToPlayerController (Pawn|GetController _aspawn)))
  (if (Pawn|IsLocalPlayerController _asplayer_controller)
    (Utilities|FlowControl|Sequence
      (:then_0
        (Utilities|IsValid _localplayerui
          (:Is%20Valid
            (Widget|RemovefromParent _localplayerui))))
      (:then_1
        (Utilities|IsValid (Actor|GetComponentbyClass _aspawn "/Script/GDKShooter.HealthComponent")
          (:Is%20Valid
            (EventDispatchers|UnbindEventfromDeath (Actor|GetComponentbyClass _aspawn "/Script/GDKShooter.HealthComponent") (EventDispatchers|CreateEvent :!event Custom|OnDeath))))))))

(event Custom|OnDeath
  (Utilities|IsValid (Variables|Default|GetLocalPlayerUI)
    (:Is%20Valid
      (Widget|RemovefromParent (Variables|Default|GetLocalPlayerUI)))))

(event EventBeginPlay
  (Utilities|FlowControl|Sequence
    (:then_0
      (Networking|SwitchHasAuthority
        (:Authority
          (bind _returnvalue (Utilities|Time|SetTimerbyEvent (EventDispatchers|CreateEvent :!event CheckControl) (Variables|Config|GetSecondsBetweenControlChecks) true))
          (Variables|Default|SetCheckControlTimerHandle _returnvalue)
          (CallFunction|FindAttachedPlayerStarts)
          (Utilities|SwitchSameTeam (Variables|Config|GetInitialControllingTeam)
            (:Different
              (CallFunction|SetStateControlled (Variables|Config|GetInitialControllingTeam)))))))
    (:then_1
      (CallFunction|MakeDynamicMaterials)
      (CallFunction|UpdateVisualsMaterial))))

(fn ConstructionScript)

(fn CheckControl
  (bind _totalsecondstoresetprogress (Variables|Config|GetTotalSecondsToResetProgress))
  (for _array_element (Collision|GetOverlappingActors (Variables|Default|GetBox) "/Game/TakeoverPrototype/BP_FPS_Character_Takeover.BP_FPS_Character_Takeover_C" :!class /Script/Engine.PrimitiveComponent)
    (bind _asbp_fps_character_takeover (Utilities|Casting|CastToBP_FPS_Character_Takeover _array_element))
    (Utilities|Array|Add (LocalVariables|GetOverlappingPlayerCharacters) _asbp_fps_character_takeover))
  (Utilities|FlowControl|Sequence
    (:then_0
      (Utilities|SwitchOverlapingPlayers
        (:Same%20Team
          (Variables|ControlState|SetIsContested false :!label _label)
          (switch Utilities|FlowControl|Switch|SwitchonEnum_ControlPointState (Variables|ControlState|GetControlState)
            (:NewEnumerator0
              ;[1 1 1] Not Controlled
              (bind _team (Utilities|SwitchOverlapingPlayers)
                (:Same%20Team
                  (CallFunction|SetStateTakingControl _team (Variables|Config|GetTotalSecondsToTakeControl)))))
            (:NewEnumerator1
              ;[1 1 1] Taking Control
              (bind _team_2 (Utilities|SwitchOverlapingPlayers)
                (:Same%20Team
                  (Utilities|SwitchSameTeam _team_2 (Variables|ControlState|GetTeamTakingControl)
                    (:Same
                      (Utilities|TickDownSecondsLeft
                        (:Finished
                          (CallFunction|SetStateControlled (Variables|ControlState|GetTeamTakingControl)))))
                    (:Different
                      (CallFunction|SetStateResettingProgress (Variables|ControlState|GetSecondsLeft) (Variables|Config|GetTotalSecondsToTakeControl)))))
                (:No%20Players
                  (CallFunction|SetStateWaitingtoResetProgress))))
            (:NewEnumerator2
              ;[1 1 1] Removing Control
              (bind _team_3 (Utilities|SwitchOverlapingPlayers)
                (:Same%20Team
                  (Utilities|SwitchSameTeam _team_3 (Variables|ControlState|GetTeamTakingControl)
                    (:Same
                      (Utilities|TickDownSecondsLeft
                        (:Finished
                          (CallFunction|SetStateNotControlled))))
                    (:Different
                      (CallFunction|SetStateResettingProgress (Variables|ControlState|GetSecondsLeft) (Variables|Config|GetTotalSecondsToRemoveControl)))))
                (:No%20Players
                  (CallFunction|SetStateWaitingtoResetProgress))))
            (:NewEnumerator3
              ;[1 1 1] Waiting to reset progress
              (bind _team_4 (Utilities|SwitchOverlapingPlayers)
                (:Same%20Team
                  (Variables|ControlState|SetResetSecondsLeft 0.0)
                  (Utilities|SwitchChangeinProgress
                    (:No%20Change
                      (Utilities|SwitchControlled
                        (:NotControlled
                          (CallFunction|SetStateTakingControl _team_4 (Variables|Config|GetTotalSecondsToTakeControl)))
                        (:Controlled
                          (CallFunction|SetStateRemovingControl _team_4 (Variables|Config|GetTotalSecondsToRemoveControl)))))
                    (:Taking%20Control
                      (Utilities|SwitchSameTeam _team_4 (Variables|ControlState|GetTeamTakingControl) :!label _label_2
                        (:Same
                          (Variables|ControlState|SetResetSecondsLeft 0.0)
                          (Utilities|SwitchChangeinProgress
                            (:Taking%20Control
                              (CallFunction|SetStateTakingControl (Variables|ControlState|GetTeamTakingControl) (Variables|ControlState|GetSecondsLeft)))
                            (:Removing%20Control
                              (CallFunction|SetStateRemovingControl (Variables|ControlState|GetTeamTakingControl) (Variables|ControlState|GetSecondsLeft)))))
                        (:Different
                          (Utilities|SwitchChangeinProgress
                            (:Taking%20Control
                              (CallFunction|SetStateResettingProgress (Variables|ControlState|GetSecondsLeft) (Variables|Config|GetTotalSecondsToTakeControl)))
                            (:Removing%20Control
                              (CallFunction|SetStateResettingProgress (Variables|ControlState|GetSecondsLeft) (Variables|Config|GetTotalSecondsToRemoveControl)))))))
                    (:Removing%20Control
                      (goto _label_2))))
                (:No%20Players
                  (Utilities|TickDownResetSecondsLeft
                    (:Finished
                      (CallFunction|SetStateResettingProgress _totalsecondstoresetprogress _totalsecondstoresetprogress))))))
            (:NewEnumerator4
              ;[1 1 1] Resetting Progress
              (Utilities|TickDownSecondsLeft
                (:Finished
                  (Utilities|SwitchControlled
                    (:NotControlled
                      (CallFunction|SetStateNotControlled))
                    (:Controlled
                      (CallFunction|SetStateControlled (Variables|Default|GetControllingTeam)))))))
            (:NewEnumerator5
              ;[1 1 1] Controlled
              (bind _team_5 (Utilities|SwitchOverlapingPlayers)
                (:Same%20Team
                  (Utilities|SwitchSameTeam _team_5 (Variables|Default|GetControllingTeam)
                    (:Different
                      (CallFunction|SetStateRemovingControl _team_5 (Variables|Config|GetTotalSecondsToRemoveControl)))))))))
        (:Different%20Teams
          (Variables|ControlState|SetIsContested true))
        (:No%20Players
          (goto _label))))
    (:then_2
      (Development|PrintText (Utilities|Text|FormatText "Controlling Team: {ControllingTeam}. State: {State}. Seconds Left. {SecondsLeft}. TeamTakingControl: {TeamTakingControl}. Reset Seconds Left: {ResetSecondsLeft} Contested: {Contested}" (.teamid (Variables|Default|GetControllingTeam)) (Utilities|Text|ToText(String) (Utilities|String|EnumtoString (Variables|ControlState|GetControlState))) (Variables|ControlState|GetSecondsLeft) (.teamid (Variables|ControlState|GetTeamTakingControl)) (Variables|ControlState|GetResetSecondsLeft) (Utilities|Text|ToText(Boolean) (Variables|ControlState|GetIsContested))) false false "(R=0.000000,G=0.660000,B=1.000000,A=1.000000)" 1.0))))

(fn ToTeams
  (params (PlayerCharacters :type Array%20of%20Actor%20Object%20References))
  (for _array_element PlayerCharacters
    (bind _asbp_fps_character (Utilities|Casting|CastToBP_FPS_Character _array_element))
    (Utilities|Array|AddUnique (LocalVariables|GetOutTeams) (Class|TeamComponent|GetTeam (Actor|GetComponentbyClass (Variables|/Script/Engine.Pawn|GetPlayerState _asbp_fps_character) "/Script/GDKShooter.TeamComponent"))))
  (return (LocalVariables|GetOutTeams)))

(fn OnRepControllingTeam
  (CallFunction|UpdateVisualsMaterial))

(fn GetTeamColour
  (params (TeamId :type Generic%20Team%20Id%20Structure))
  (return (Math|Color|SelectColor "(R=1.000000,G=1.000000,B=1.000000,A=1.000000)" (Math|Color|SelectColor "(R=0.812500,G=0.000000,B=0.000000,A=1.000000)" "(R=0.014625,G=0.159246,B=0.859375,A=1.000000)" (== (.teamid TeamId) 0)) (== (.teamid TeamId) 255))))

(fn IsControlled
  (Utilities|SwitchControlled
    (:NotControlled
      (return false))
    (:Controlled
      (return true))))

(fn IsChangeinProgress
  (Utilities|SwitchSameTeam (Variables|ControlState|GetTeamTakingControl)
    (:Same
      (return false false))
    (:Different
      (Utilities|SwitchControlled
        (:NotControlled
          (return true true))
        (:Controlled
          (return true false))))))

(fn FindAttachedPlayerStarts
  (for _array_element (Actor|GetAttachedActors true)
    (bind _asteam_player_start (Utilities|Casting|CastToTeamPlayerStart _array_element))
    (Utilities|Array|Add (Variables|Default|GetPlayerStarts) _asteam_player_start)))

(fn SetControlState
  (params (NewState :type Enum_ControlPointState%20Enum :default "NewEnumerator0"))
  (Variables|ControlState|SetControlState NewState)
  (CallFunction|UpdatePlayerStartsTeam))

(fn UpdatePlayerStartsTeam
  (for _array_element (Actor|GetAttachedActors true)
    (Utilities|IsValid (Actor|GetComponentbyClass _array_element "/Script/GDKShooter.TeamComponent")
      (:Is%20Valid
        (Class|TeamComponent|SetTeam (Actor|GetComponentbyClass _array_element "/Script/GDKShooter.TeamComponent") (Variables|Default|GetControllingTeam))))))

(fn SetStateTakingControl
  (params (TeamTakingControl :type Generic%20Team%20Id%20Structure) (SecondsLeft :type Float%20%28single-precision%29))
  (Variables|ControlState|SetSecondsLeft SecondsLeft)
  (Variables|ControlState|SetTeamTakingControl TeamTakingControl)
  (CallFunction|SetControlState "NewEnumerator1"))

(fn SetStateRemovingControl
  (params (TeamRemovingControl :type Generic%20Team%20Id%20Structure) (SecondsLeft :type Float%20%28single-precision%29))
  (Variables|ControlState|SetSecondsLeft SecondsLeft)
  (Variables|ControlState|SetTeamTakingControl TeamRemovingControl)
  (CallFunction|SetControlState "NewEnumerator2"))

(fn SetStateControlled
  (params (ControllingTeam :type Generic%20Team%20Id%20Structure))
  (Variables|Default|SetControllingTeam ControllingTeam)
  (Variables|ControlState|SetTeamTakingControl (Utilities|Struct|MakeGenericTeamId 255))
  (Variables|ControlState|SetControlState "NewEnumerator5")
  (CallFunction|UpdatePlayerStartsTeam)
  (Default|CallOnControllingTeamChanged))

(fn SetStateNotControlled
  (Variables|Default|SetControllingTeam (Utilities|Struct|MakeGenericTeamId 255))
  (Variables|ControlState|SetControlState "NewEnumerator0")
  (CallFunction|UpdatePlayerStartsTeam)
  (Default|CallOnControllingTeamChanged))

(fn SetStateResettingProgress
  (params (SecondsLeft :type Float%20%28single-precision%29) (Total :type Float%20%28single-precision%29))
  (Variables|ControlState|SetSecondsLeft (* (Variables|Config|GetTotalSecondsToResetProgress) (- 1.0 (/ SecondsLeft Total)))) ; Time to reset is proportional to amount of progress made taking control
  (Variables|ControlState|SetControlState "NewEnumerator4"))

(fn SetStateWaitingtoResetProgress
  (Variables|ControlState|SetResetSecondsLeft (Variables|Config|GetTotalSecondsBeforeProgressResets))
  (CallFunction|SetControlState "NewEnumerator3"))

(fn UpdateVisualsMaterial
  (for _array_element (Utilities|Array|MakeArray (Variables|Default|GetVisuals) (Variables|Default|GetLightShaft))
    (bind _asmaterial_instance_dynamic (Utilities|Casting|CastToMaterialInstanceDynamic (Rendering|Material|GetMaterial _array_element 0)))
    (Rendering|Material|SetVectorParameterValue _asmaterial_instance_dynamic "Colour" (CallFunction|GetTeamColour (Variables|Default|GetControllingTeam)) :!class /Script/Engine.MaterialInstanceDynamic)))

(fn MakeDynamicMaterials
  (for _array_element (Utilities|Array|MakeArray (Variables|Default|GetVisuals) (Variables|Default|GetLightShaft))
    (bind _returnvalue (Rendering|Material|CreateDynamicMaterialInstance _array_element 0 (Rendering|Material|GetMaterial _array_element 0) "None" :!class /Script/Engine.PrimitiveComponent))
    (Rendering|Material|SetMaterial _array_element 0 _returnvalue)))