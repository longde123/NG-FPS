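; Base character Blueprint handling held items, death and an in-world nameplate.
; Equipped component changes attach holdables to mesh sockets, and gaining authority spawns starter templates from metadata.
; Health events drive dynamic nameplate and mesh materials, while death ragdolls with a directional impulse, with authoritative death also setting a lifespan.
; Hover fades in the nameplate briefly via timeline and timer, and team changes re-register the AI perception stimuli source.
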(event TeamChanged(TeamComponent)
  (params (Team :type Generic%20Team%20Id%20Structure))
  (Class|AIPerceptionStimuliSourceComponent|UnregisterfromPerceptionSystem (Variables|Default|GetAIPerceptionStimuliSource))
  (Utilities|FlowControl|Delay 0.2)
  (Class|AIPerceptionStimuliSourceComponent|RegisterwithPerceptionSystem (Variables|Default|GetAIPerceptionStimuliSource)))

(event AuthoritativeDeath(HealthComponent)
  (params (Instigator :type Controller%20Object%20Reference))
  ;[1 1 1] Authoritative Death, Ragdoll, Set Lifespan
  (Class|GDKCharacter|StartRagdoll)
  (Actor|SetLifeSpan 1e+01))

(event ArmourUpdated(HealthComponent)
  (params (Current :type Float%20%28single-precision%29) (Max :type Float%20%28single-precision%29))
  ;[1 1 1] Set Nameplate Armour
  (bind _nameplatematerial (Variables|Default|GetNameplateMaterial)
    (:then
      (Rendering|Material|SetScalarParameterValue _nameplatematerial "Armour" (/ Current Max) :!class /Script/Engine.MaterialInstanceDynamic))
    (:else)))

(event HealthUpdated(HealthComponent)
  (params (Current :type Float%20%28single-precision%29) (Max :type Float%20%28single-precision%29))
  ;[1 1 1] Set Nameplate and Mesh Material Health
  (CallFunction|UpdateHealthMaterialValues Current Max))

(event Death(HealthComponent)
  (bind _equippedcomponent (Variables|Default|GetEquippedComponent))
  (bind _returnvalue (Class|EquippedComponent|CurrentlyHeldItem _equippedcomponent))
  ;[1 1 1] NonAuthoritative Death, Stop Shooting and Ragdoll
  (Utilities|IsValid _returnvalue
    (:Is%20Valid
      (Class|Holdable|StopPrimaryUse _returnvalue)
      (Class|Holdable|StopSecondaryUse _returnvalue))
    (:Is%20Not%20Valid
      _))
  (Utilities|FlowControl|Delay 0.2)
  (Class|GDKCharacter|StartRagdoll)
  (CallFunction|HoverHide))

(event Custom|HoverExpire
  ;[1 1 1] Hover Logic for dispaying nameplates only shortly after the crosshair passes over a character
  (bind (_direction _nameplateopacity) (Timeline|NameplateOpacity Reverse)
    (:Update
      (Rendering|Material|SetScalarParameterValue (Variables|Default|GetNameplateMaterial) "Opacity" _nameplateopacity :!class /Script/Engine.MaterialInstanceDynamic))
    (:Finished
      (if (Utilities|Enum|Equal(Enum) _direction "Backward")
        (Rendering|SetVisibility (Variables|Default|GetNameplate) false false)))))

(event Custom|HoverHide
  ;[1 1 1] Hover Logic for dispaying nameplates only shortly after the crosshair passes over a character
  (bind (_direction _nameplateopacity) (Timeline|NameplateOpacity Reverse)
    (:Update
      (Rendering|Material|SetScalarParameterValue (Variables|Default|GetNameplateMaterial) "Opacity" _nameplateopacity :!class /Script/Engine.MaterialInstanceDynamic))
    (:Finished
      (if (Utilities|Enum|Equal(Enum) _direction "Backward")
        (Rendering|SetVisibility (Variables|Default|GetNameplate) false false)))))

(event Custom|SetPlayerName
  (bind _playerstate (Variables|Default|GetPlayerState))
  (bind _nameplatematerial (Variables|Default|GetNameplateMaterial))
  ;[1 1 1] Try to get the player name from the player state
  (Utilities|IsValid _playerstate
    (:Is%20Valid
      (Variables|Default|SetPlayerName (PlayerState|GetPlayerName _playerstate)))
    (:Is%20Not%20Valid
      (Variables|Default|SetPlayerName (Utilities|GetDisplayName self))))
  (bind _nameplate (Variables|Default|GetNameplate)
    (:then
      (Rendering|Components|TextRender|SetText _nameplate (Utilities|Text|ToText(String) (Variables|Default|GetPlayerName)))
      (Rendering|Material|SetScalarParameterValue _nameplatematerial "TextWidth" (.y (Class|TextRenderComponent|GetTextLocalSize _nameplate)) :!class /Script/Engine.MaterialInstanceDynamic)
      (Rendering|Material|SetScalarParameterValue _nameplatematerial "TextHeight" (.z (Class|TextRenderComponent|GetTextLocalSize _nameplate)) :!class /Script/Engine.MaterialInstanceDynamic))
    (:else)))

(event EventOnHover
  ;[1 1 1] Hover Logic for dispaying nameplates only shortly after the crosshair passes over a character
  (if (> (Class|HealthComponent|GetCurrentHealth (Variables|Default|GetHealthComponent)) 0.0)
    (CallFunction|SetPlayerName)
    (bind _nameplate (Variables|Default|GetNameplate)
      (:then
        (Rendering|SetVisibility _nameplate true false)
        (Utilities|Time|SetTimerbyEvent (delegate Custom|HoverExpire) 2.0)
        (bind (_direction _nameplateopacity) (Timeline|NameplateOpacity Play)
          (:Update
            (Rendering|Material|SetScalarParameterValue (Variables|Default|GetNameplateMaterial) "Opacity" _nameplateopacity :!class /Script/Engine.MaterialInstanceDynamic))
          (:Finished
            (if (Utilities|Enum|Equal(Enum) _direction "Backward")
              (Rendering|SetVisibility (Variables|Default|GetNameplate) false false)))))
      (:else))))

(event EventOnEquippedUpdated
  (params (NewHoldable :type Holdable%20Object%20Reference))
  (CallFunction|AttachHoldable NewHoldable))

(event EventStartRagdoll
  ;[1 1 1] Launch Ragdoll on death
  (|CallParentFunction)
  (Physics|AddImpulse (Variables|Character|GetMesh) (* (+ (Math|Vector|Normalize (Variables|Default|GetLastDamageDirection)) "0, 0,0.200000") (Variables|Default|GetLaunchStrength)) "Hips" false))

(event EventAuthorityGained
  (Class|EquippedComponent|SpawnStarterTemplates (Variables|Default|GetEquippedComponent) (Variables|/Script/GDKShooter.MetaDataComponent|GetMetaData (Variables|Default|GetMetaDataComponent))))

(event EventBeginPlay
  (|CallParentFunction)
  (CallFunction|AttachHoldable (Class|EquippedComponent|CurrentlyHeldItem (Variables|Default|GetEquippedComponent))))

(fn ConstructionScript
  (bind _nameplate (Variables|Default|GetNameplate)
    (:then
      (bind _returnvalue (Rendering|Material|CreateDynamicMaterialInstance _nameplate 0 0 "None" :!class /Script/Engine.PrimitiveComponent))
      (Variables|Default|SetNameplateMaterial _returnvalue)
      (bind _returnvalue_2 (Rendering|Material|CreateDynamicMaterialInstance (Variables|Character|GetMesh) 0 0 "None" :!class /Script/Engine.PrimitiveComponent))
      (Variables|Default|SetMeshMaterial _returnvalue_2))
    (:else)))

(fn UpdateHealthMaterialValues
  (params (Current :type Float%20%28single-precision%29) (Max :type Float%20%28single-precision%29))
  (bind _returnvalue (/ Current Max))
  (bind _meshmaterial (Variables|Default|GetMeshMaterial))
  (bind _nameplatematerial (Variables|Default|GetNameplateMaterial)
    (:then
      (Rendering|Material|SetScalarParameterValue _nameplatematerial "Health" _returnvalue :!class /Script/Engine.MaterialInstanceDynamic)
      (Utilities|IsValid _meshmaterial
        (:Is%20Valid
          (Rendering|Material|SetScalarParameterValue _meshmaterial "Health" _returnvalue :!class /Script/Engine.MaterialInstanceDynamic))))
    (:else)))

(fn AttachHoldable
  (params (CurrentHoldable :type Holdable%20Object%20Reference))
  (Utilities|IsValid CurrentHoldable
    (:Is%20Valid
      (Transformation|AttachComponentToComponent CurrentHoldable (Variables|Character|GetMesh) (Class|Holdable|GetActiveSocket CurrentHoldable) "SnapToTarget" "SnapToTarget" "KeepRelative" true))))